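; BP_Wind is a wind controller actor for the Abandoned Cathedral foliage content that feeds global wind values to materials.
; It writes its Intensity and Speed variables, plus the root component's forward vector as wind direction, into the MP_master_Parameter material parameter collection.
; The same writes run in the Construction Script and on every Tick, so rotating the actor sets the wind direction both in the editor and at runtime.
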(event `self.ReceiveTick`
  (params (DeltaSeconds :type "Float (single-precision)"))
  (`KismetMaterialLibrary.SetScalarParameterValue` "/Game/Abandoned_Cathedral/Foliage/Master_Parameter/MP_master_Parameter.MP_master_Parameter" "WindINT" (`self.Intensity`))
  (`KismetMaterialLibrary.SetScalarParameterValue` "/Game/Abandoned_Cathedral/Foliage/Master_Parameter/MP_master_Parameter.MP_master_Parameter" "WindSpeed" (`self.Speed`))
  (`KismetMaterialLibrary.SetVectorParameterValue` "/Game/Abandoned_Cathedral/Foliage/Master_Parameter/MP_master_Parameter.MP_master_Parameter" "WindDirection" (`KismetMathLibrary.Conv_VectorToLinearColor` (`SceneComponent.GetForwardVector` (`self.DefaultSceneRoot`)))))

(fn `UserConstructionScript`
  (`KismetMaterialLibrary.SetScalarParameterValue` "/Game/Abandoned_Cathedral/Foliage/Master_Parameter/MP_master_Parameter.MP_master_Parameter" "WindINT" (`self.Intensity`))
  (`KismetMaterialLibrary.SetScalarParameterValue` "/Game/Abandoned_Cathedral/Foliage/Master_Parameter/MP_master_Parameter.MP_master_Parameter" "WindSpeed" (`self.Speed`))
  (`KismetMaterialLibrary.SetVectorParameterValue` "/Game/Abandoned_Cathedral/Foliage/Master_Parameter/MP_master_Parameter.MP_master_Parameter" "WindDirection" (`KismetMathLibrary.Conv_VectorToLinearColor` (`SceneComponent.GetForwardVector` (`self.DefaultSceneRoot`)))))