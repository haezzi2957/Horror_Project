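; BP_MasterItem is an interactable item, likely a base class, that shows an interaction hint to the player.
; While CanInteract is set, its sphere overlap creates or removes a UI_Interact widget, with an animated pop-up and mesh outline overlay.
; A CanReceiveTrace event also toggles the hint on an existing widget, using another outline material.
; HintVisible guards against replays, and CanPressE flags readiness for input, which is handled outside this graph.
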(event `self.Sphere.OnComponentBeginOverlap`
  (params (OverlappedComponent :type "PrimitiveComponent Object Reference") (OtherActor :type "Actor Object Reference") (OtherComp :type "PrimitiveComponent Object Reference") (OtherBodyIndex :type Integer) (bFromSweep :type Boolean) (SweepResult :type "HitResult Structure (by ref)"))
  (bind _widget (`self.Widget`))
  (cast `/Game/BluePrints/BP_PlayerCharacter` OtherActor)
  (if (`self.CanInteract`)
    (bind _returnvalue (`|CreateWidget` "/Game/UI/UI_Interact.UI_Interact_C"))
    (bind _output_get (set `self.Interaction Widget` _returnvalue))
    (`WidgetComponent.SetWidget` _widget _output_get)
    (`SceneComponent.SetVisibility` _widget true false)
    (bind _interaction_widget (`self.Interaction Widget`)
      (:`then`
        (if (not (`self.HintVisible`))
          (`UserWidget.PlayAnimation` _interaction_widget (`/Game/UI/UI_Interact.PopUp` _interaction_widget) 0.0 1 "Forward" 1.5 false)
          (set `self.HintVisible` true)
          (`MeshComponent.SetOverlayMaterial` (`self.StaticMesh`) "/Game/UI/M_Outline.M_Outline")
          (set `self.CanPressE` true)))
      (:`else`))))

(event `self.Sphere.OnComponentEndOverlap`
  (params (OverlappedComponent :type "PrimitiveComponent Object Reference") (OtherActor :type "Actor Object Reference") (OtherComp :type "PrimitiveComponent Object Reference") (OtherBodyIndex :type Integer))
  (cast `/Game/BluePrints/BP_PlayerCharacter` OtherActor)
  (if (`self.CanInteract`)
    (bind _interaction_widget (`self.Interaction Widget`)
      (:`then`
        (if (`self.HintVisible`)
          (`UserWidget.PlayAnimation` _interaction_widget (`/Game/UI/UI_Interact.PopUp` _interaction_widget) 0.0 1 "Reverse" 1.5 false)
          (set `self.HintVisible` false)
          (set `self.CanPressE` false)
          (`MeshComponent.SetOverlayMaterial` (`self.StaticMesh`) null))
        (`KismetSystemLibrary.Delay` 0.15)
        (`Widget.RemoveFromParent` (`self.Interaction Widget`))
        (set `self.Interaction Widget` null)
        (`SceneComponent.SetVisibility` (`self.Widget`) false false))
      (:`else`))))

(event `/Game/UI/BPI_Interaction.Can Receive Trace`
  (params (`Can Interact` :type Boolean))
  (if (`self.CanInteract`)
    (if `Can Interact`
      (bind _interaction_widget (`self.Interaction Widget`)
        (:`then`
          (if (not (`self.HintVisible`))
            (`UserWidget.PlayAnimation` _interaction_widget (`/Game/UI/UI_Interact.PopUp` _interaction_widget) 0.0 1 "Forward" 1.5 false)
            (set `self.HintVisible` true)
            (`MeshComponent.SetOverlayMaterial` (`self.StaticMesh`) "/Game/UI/MI_Outline1.MI_Outline1")
            (set `self.CanPressE` true)))
        (:`else`))
      (else
        (bind _interaction_widget_2 (`self.Interaction Widget`)
          (:`then`
            (if (`self.HintVisible`)
              (`UserWidget.PlayAnimation` _interaction_widget_2 (`/Game/UI/UI_Interact.PopUp` _interaction_widget_2) 0.0 1 "Reverse" 1.5 false)
              (set `self.HintVisible` false)
              (`MeshComponent.SetOverlayMaterial` (`self.StaticMesh`) null)
              (set `self.CanPressE` false)))
          (:`else`))))))

(fn `UserConstructionScript`)