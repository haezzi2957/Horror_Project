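; Player character Blueprint that handles interaction, the HUD and an attached flashlight.
; BeginPlay creates the HUD, attaches a spawned flashlight to a mesh socket and starts fast looping timers for camera shakes and interaction tracing.
; A camera-forward sphere trace caches the BPI_Interaction actor as TraceItem and messages it on focus or when nothing interactable is hit.
; E sends InteractMessage to that item, and IA_Flashlight toggles the flashlight.
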(event `Create Interaction Trace`
  (`self.Interaction Trace`))

(event `Key|E`
  (params (Key :type "Key Structure"))
  (:`Pressed`
    (message `/Game/UI/BPI_Interaction.Interact` (`self.Trace Item`))))

(event `self.ReceiveBeginPlay`
  (`|ExecutionSequence`
    (:`then_0`
      (`KismetSystemLibrary.K2_SetTimer` null "SetCameraShakes" 0.01 true)
      (bind _returnvalue (`KismetSystemLibrary.K2_SetTimer` null "Create Interaction Trace" 0.01 true))
      (set `self.Interaction Timer` _returnvalue)
      (bind _returnvalue_2 (`|CreateWidget` "/Game/UI/UI_HUD.UI_HUD_C"))
      (`UserWidget.AddToViewport` _returnvalue_2 0))
    (:`then_1`
      (bind _returnvalue_3 (`|SpawnActorFromClass` "/Game/BluePrints/BP_Flashlight.BP_Flashlight_C" (`SceneComponent.K2_GetComponentToWorld` (`self.Mesh`)) "Undefined" "MultiplyWithRoot" null null))
      (bind _output_get (set `self.Flashlight_0` _returnvalue_3))
      (`self.K2_AttachToComponent` _output_get (`self.Mesh`) "Flashlight_Socket" "SnapToTarget" "SnapToTarget" "SnapToTarget" false))))

(event `EnhancedInput|/Game/FPFlashlightAnims/Demo/Player/FirstPerson/Input/Actions/IA_Flashlight`
  (params (ActionValue :type Boolean) (ElapsedSeconds :type "Float (double-precision)") (TriggeredSeconds :type "Float (double-precision)") (InputAction :type "InputAction Object Reference" :default "/Game/FPFlashlightAnims/Demo/Player/FirstPerson/Input/Actions/IA_Flashlight.IA_Flashlight"))
  (:`Triggered`
    (`self.FlashlightToggle`)
    (`/Game/BluePrints/BP_Flashlight.ToggleFlashlight` (`self.Flashlight_0`))))

(fn `Interaction Trace`
  (bind _camera (`self.Camera`))
  (bind _returnvalue (`SceneComponent.K2_GetComponentLocation` _camera))
  (bind _outhit (`KismetSystemLibrary.SphereTraceSingle` _returnvalue (+ _returnvalue (* (`KismetMathLibrary.GetForwardVector` (`SceneComponent.K2_GetComponentRotation` _camera)) 1000.0)) 3.0 "TraceTypeQuery1"))
  (bind (_bblockinghit _binitialoverlap _time _distance _location _impactpoint _normal _impactnormal _physmat _hitactor) (`GameplayStatics.BreakHitResult` _outhit))
  (if (`KismetSystemLibrary.DoesImplementInterface` _hitactor "/Game/UI/BPI_Interaction.BPI_Interaction_C")
    (if (!= _hitactor (`self.Trace Item`))
      (bind _output_get (set `self.Trace Item` _hitactor))
      (message `/Game/UI/BPI_Interaction.Can Receive Trace` _output_get true))
    (else
      (message `/Game/UI/BPI_Interaction.Can Receive Trace` (`self.Trace Item`) false)
      (set `self.Trace Item` null))))

(fn `UserConstructionScript`)