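; BP_Switch is an interactable switch that toggles the visibility of a referenced light's component.
; Its Interact event acts only while CanPressE and CanInteract are both true, clearing CanInteract as it starts.
; Turning the light on restores CanInteract, while turning it off leaves it false, blocking further presses unless it is reset elsewhere.
; The construction script only calls its parent.
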(event `/Game/UI/BPI_Interaction.Interact`
  (bind _lightcomponent (`Light.LightComponent` (`self.Light`)))
  (if (`self.CanPressE`)
    (if (`self.CanInteract`)
      (set `self.CanInteract` false)
      (if (`SceneComponent.bVisible` _lightcomponent)
        (`SceneComponent.SetVisibility` _lightcomponent false false)
        (set `self.CanInteract` false)
        (else
          (`SceneComponent.SetVisibility` _lightcomponent true false)
          (set `self.CanInteract` true))))))

(fn `UserConstructionScript`
  (`parent.UserConstructionScript`))